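; GA_Roll is a Gameplay Ability that performs the main character's dodge roll, with a window of invulnerability.
; On activation it disables player input, stops movement and plays the roll montage.
; AnimNotify gameplay events bound the roll: AbilityBegin adds the invulnerability tag and a forward root motion constant force, while AbilityEnd removes the tag, restores input and ends the force.
; The montage finishing or being interrupted ends the ability, which also re-enables input.
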(event Custom|Initialize)

(event Ability|EventActivateAbility
  (Ability|CommitAbility)
  (if true
    (bind _asbp_main_character (Utilities|Casting|CastToBP_MainCharacter (Ability|GetOwningActorfromActorInfo))
      (:then
        (bind _output_get (Variables|Default|SetMainCharacter _asbp_main_character))
        (bind _aspc_main_character_controller (Utilities|Casting|CastToPC_MainCharacterController (Pawn|GetController _output_get))
          (:then
            (bind _output_get_2 (Variables|Default|SetCharacterController _aspc_main_character_controller))
            (Input|DisableInput _output_get_2 _output_get_2)
            (Components|Movement|StopMovementImmediately (Variables|/Script/Engine.Character|GetCharacterMovement (Variables|Default|GetMainCharacter)))
            (|PlayMontageandWaitProxy "None" "/Game/Mannequin/Montages/AM_Roll.AM_Roll" 2.0 "None" true 1.0 0.0
              (:then
                (Ability|Tasks|WaitGameplayEvent "(TagName=\"AnimNotify.AbilityBegin\")" 0
                  (:EventReceived
                    (Ability|GameplayEffect|AddLooseGameplayTags (Variables|Default|GetMainCharacter) (GameplayTags|MakeGameplayTagContainerfromTag (Variables|Default|GetInvulnerabilityTag)))
                    (bind _asynctaskproxy (Ability|Tasks|ApplyRootMotionConstantForce "None" (Math|Rotator|GetRotationXVector (Transformation|GetActorRotation (Variables|Default|GetMainCharacter))) (Variables|Default|GetRollSpeed) 1e+01 true 0 "SetVelocity")
                      (:then
                        (Variables|Default|SetRootMotionTask _asynctaskproxy)
                        (Ability|Tasks|WaitGameplayEvent "(TagName=\"AnimNotify.AbilityEnd\")" 0
                          (:EventReceived
                            (Ability|GameplayEffect|RemoveLooseGameplayTags (Variables|Default|GetMainCharacter) (GameplayTags|MakeGameplayTagContainerfromTag (Variables|Default|GetInvulnerabilityTag)))
                            (Utilities|IsValid (Variables|Default|GetCharacterController)
                              (:Is%20Valid
                                (Input|EnableInput (Variables|Default|GetCharacterController) (Variables|Default|GetCharacterController))
                                (Utilities|IsValid (Variables|Default|GetRootMotionTask)
                                  (:Is%20Valid
                                    (GameplayTasks|EndTask (Variables|Default|GetRootMotionTask)))))))))))))
              (:OnCompleted
                (Ability|EndAbility :!label _label))
              (:OnBlendOut
                (goto _label))
              (:OnInterrupted
                (goto _label))
              (:OnCancelled
                (goto _label))))
          (:CastFailed
            (Ability|EndAbility :!label _label_2))))
      (:CastFailed
        (goto _label_2)))
    (else
      (goto _label_2))))

(event Ability|EventOnEndAbility
  (params (bWasCancelled :type Boolean))
  (bind _charactercontroller (Variables|Default|GetCharacterController))
  (Utilities|IsValid _charactercontroller
    (:Is%20Valid
      (Input|EnableInput _charactercontroller _charactercontroller))))