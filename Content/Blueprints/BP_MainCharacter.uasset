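; BP_MainCharacter is the main character Blueprint, with hotkeys that apply health and mana potion effects through the Gameplay Ability System.
; Keys 2 and 3 build a spec for GE_HealthPotion or GE_ManaPotion, set a fixed magnitude by tag (SetByCaller), and apply it to the character's own Ability System Component.
; Key 1 only triggers a FlipFlop with no connected outputs, and an Inventory node is unused.
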(event Input|KeyboardEvents|1
  (params (Key :type Key%20Structure :default "None"))
  (:Pressed
    (Utilities|FlowControl|FlipFlop)))

(event Input|KeyboardEvents|2
  (params (Key :type Key%20Structure :default "None"))
  (bind _self self)
  (bind _returnvalue (Ability|GetAbilitySystemComponent _self))
  (:Pressed
    (bind _returnvalue_2 (Ability|GameplayEffect|AssignTagSetbyCallerMagnitude (GameplayEffects|MakeOutgoingSpec _returnvalue "/Game/GAS/GameplayEffects/GE_HealthPotion.GE_HealthPotion_C" 0.0 (Utilities|Struct|MakeGameplayEffectContextHandle)) "(TagName=\"Attribute.Health.HealPotion\")" 2e+01))
    (GameplayEffects|ApplyGameplayEffectSpecToSelf _returnvalue _returnvalue_2)))

(event Input|KeyboardEvents|3
  (params (Key :type Key%20Structure :default "None"))
  (bind _self self)
  (bind _returnvalue (Ability|GetAbilitySystemComponent _self))
  (:Pressed
    (bind _returnvalue_2 (Ability|GameplayEffect|AssignTagSetbyCallerMagnitude (GameplayEffects|MakeOutgoingSpec _returnvalue "/Game/GAS/GameplayEffects/GE_ManaPotion.GE_ManaPotion_C" 0.0 (Utilities|Struct|MakeGameplayEffectContextHandle)) "(TagName=\"Attribute.Mana.ManaPotion\")" 4e+01))
    (GameplayEffects|ApplyGameplayEffectSpecToSelf _returnvalue _returnvalue_2)))

(fn ConstructionScript)